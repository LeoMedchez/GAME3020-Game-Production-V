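; Interactable barrier gate that the player opens and closes with E while inside its trigger box.
; Overlap by BP_PlayerCharacter enables or disables the actor's input for player controller 0.
; Opening slides the lock bolt by timeline, then swings RotatePoint to OpenAngle after a delay.
; Closing reverses both timelines in the opposite order, with delays before IsClosed updates.
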(event `GateOpen`
  (bind (_direction _alpha) (`Timeline|OpenGate` :!label _label)
    (:`Update`
      (`SceneComponent.K2_SetRelativeRotation` (`self.RotatePoint`) (`KismetMathLibrary.RLerp` (struct) (`self.Open Angle`) _alpha) false false))))

(event `LockOpen`
  (bind (_direction _alpha) (`Timeline|TL_Bolt` :!label _label_2)
    (:`Update`
      (`SceneComponent.K2_SetRelativeLocation` (`self.Lock`) (`KismetMathLibrary.VLerp` (0.0 0.0 0.0) (-6.0 0.0 0.0) _alpha) false false))))

(event `GateClose`
  (goto _label :!via `Reverse`))

(event `LockClose`
  (goto _label_2 :!via `Reverse`))

(event `Key|E`
  (params (Key :type "Key Structure"))
  (:`Pressed`
    (if (`self.IsClosed`)
      (`self.LockOpen`)
      (`KismetSystemLibrary.Delay` 1.0)
      (`self.GateOpen`)
      (set `self.IsClosed` false)
      (else
        (`self.GateClose`)
        (`KismetSystemLibrary.Delay` 2.5)
        (`self.LockClose`)
        (`KismetSystemLibrary.Delay` 0.75)
        (set `self.IsClosed` true)))))

(event `self.Box.OnComponentBeginOverlap`
  (params (OverlappedComponent :type "PrimitiveComponent Object Reference") (OtherActor :type "Actor Object Reference") (OtherComp :type "PrimitiveComponent Object Reference") (OtherBodyIndex :type Integer) (bFromSweep :type Boolean) (SweepResult :type "HitResult Structure (by ref)"))
  (cast `/Game/Characters/Player_Character/BP_PlayerCharacter` OtherActor)
  (`self.EnableInput` (`GameplayStatics.GetPlayerController` 0)))

(event `self.Box.OnComponentEndOverlap`
  (params (OverlappedComponent :type "PrimitiveComponent Object Reference") (OtherActor :type "Actor Object Reference") (OtherComp :type "PrimitiveComponent Object Reference") (OtherBodyIndex :type Integer))
  (cast `/Game/Characters/Player_Character/BP_PlayerCharacter` OtherActor)
  (`self.DisableInput` (`GameplayStatics.GetPlayerController` 0)))

(fn `UserConstructionScript`)