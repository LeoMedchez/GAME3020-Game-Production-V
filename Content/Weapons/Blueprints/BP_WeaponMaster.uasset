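; BP_WeaponMaster is a weapon Blueprint with a pickup prompt and a laser beam.
; Box overlap events toggle InPickupRange and show or remove a WBP_PressToPickup widget, with no filter on the overlapping actor.
; Each Tick moves the Niagara beam to LaserSocket and line-traces along the mesh's right vector on Visibility.
; The beam's end parameter is set to the impact point, or to the trace end when nothing blocks it.
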(event `self.Box.OnComponentBeginOverlap`
  (params (OverlappedComponent :type "PrimitiveComponent Object Reference") (OtherActor :type "Actor Object Reference") (OtherComp :type "PrimitiveComponent Object Reference") (OtherBodyIndex :type Integer) (bFromSweep :type Boolean) (SweepResult :type "HitResult Structure (by ref)"))
  (set `self.InPickupRange` true)
  (bind _returnvalue (`|CreateWidget` "/Game/Blueprints/UI/WBP_PressToPickup.WBP_PressToPickup_C" (`GameplayStatics.GetPlayerController` 0)))
  (bind _output_get (set `self.PickupWidgetRef` _returnvalue))
  (`UserWidget.AddToViewport` _output_get 0))

(event `self.Box.OnComponentEndOverlap`
  (params (OverlappedComponent :type "PrimitiveComponent Object Reference") (OtherActor :type "Actor Object Reference") (OtherComp :type "PrimitiveComponent Object Reference") (OtherBodyIndex :type Integer))
  (set `self.InPickupRange` false)
  (`Widget.RemoveFromParent` (`self.PickupWidgetRef`)))

(event `self.ReceiveTick`
  (params (DeltaSeconds :type "Float (single-precision)"))
  (bind _returnvalue (`SceneComponent.GetSocketLocation` (`self.Weapon_SK`) (`self.Laser Socket`)))
  (`SceneComponent.K2_SetWorldLocation` (`self.NS_LaserBeam`) (`SceneComponent.GetSocketLocation` (`self.Weapon_SK`) (`self.Laser Socket`)) false false)
  (bind _outhit (`KismetSystemLibrary.LineTraceSingle` _returnvalue (+ _returnvalue (* (`SceneComponent.GetRightVector` (`self.Weapon_SK`)) 1500.0)) "TraceTypeQuery1"))
  (bind (_bblockinghit _binitialoverlap _time _distance _location _impactpoint _normal _impactnormal _physmat _hitactor _hitcomponent _hitbonename _bonename _hititem _elementindex _faceindex _tracestart _traceend) (`GameplayStatics.BreakHitResult` _outhit))
  (`FXSystemComponent.SetVectorParameter` (`self.NS_LaserBeam`) "Beam End" (`KismetMathLibrary.SelectVector` _impactpoint _traceend _bblockinghit)))

(fn `UserConstructionScript`)